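; BP_PlayerSprite is the side-scrolling Paper2D player character, handling run, jump, crouch and pausing through Enhanced Input.
; Each tick it picks the idle, run, jump, fall or crouch flipbook from movement state and flips control yaw by X velocity.
; Crouch is a manual toggle of IsCrouching and max walk speed instead of the built-in Crouch functions.
; Pause opens the PauseMenu widget, switches to UI-only input and pauses the game.
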(event Custom|UpdateAnimation
  ;[0.3694 0.7653 1] Changing the sprite's anaimtion determined by the character's movment
  (Sprite|SetFlipbook (Variables|Default|GetSprite) (select (Variables|Default|GetisCrouching) "/Game/Art/SunnyLand/sprites/player/crouch/FB_player-crouch.FB_player-crouch" (select (> (.Z (Math|Vector|BreakVector (Variables|/Script/Engine.MovementComponent|GetVelocity (Variables|Character|GetCharacterMovement)))) 1.0) "/Game/Art/SunnyLand/sprites/player/jump/FB_player-jump.FB_player-jump" (select (AI|Components|NavMovement|IsFalling (Variables|Character|GetCharacterMovement)) "/Game/Art/SunnyLand/sprites/player/jump/FB_player-fall.FB_player-fall" (select (> (Math|Vector|VectorLength (Variables|/Script/Engine.MovementComponent|GetVelocity (Variables|Character|GetCharacterMovement))) 0.0) "/Game/Art/SunnyLand/sprites/player/run/FB_player-run.FB_player-run" "/Game/Art/SunnyLand/sprites/player/idle/FB_player-idle.FB_player-idle"))))))

(event Custom|UpdateDirection
  ;[1 0.4402 0.8601] Changing the direction of the sprite
  (Utilities|IsValid (Pawn|GetController)
    (:Is%20Valid
      (Math|Float|CompareFloat (.X (Math|Vector|BreakVector (Variables|/Script/Engine.MovementComponent|GetVelocity (Variables|Character|GetCharacterMovement)))) 0.0
        (:>
          (Pawn|SetControlRotation (Pawn|GetController) (Math|Rotator|MakeRotator 0.0 0.0 0.0)))
        (:<
          (Pawn|SetControlRotation (Pawn|GetController) (Math|Rotator|MakeRotator 0.0 0.0 1.8e+02)))))))

(event Custom|ToggleCrouch
  (params (Crouch :type Boolean))
  ;[1 0.06771 0.06771] Toggle Crouch, Setting the Movement Settings Since "Crouch" and "Un Crouch" won't work >:(
  (if Crouch
    (Variables|/Script/Engine.CharacterMovementComponent|SetMaxWalkSpeed (Variables|Character|GetCharacterMovement) (Variables|Default|GetcrouchSpeed))
    (Variables|Default|SetisCrouching true)
    (else
      (Variables|/Script/Engine.CharacterMovementComponent|SetMaxWalkSpeed (Variables|Character|GetCharacterMovement) (Variables|Default|GetwalkSpeed))
      (Variables|Default|SetisCrouching false))))

(event Input|EnhancedActionEvents|EnhancedInputActionIA_Jump
  (params (ActionValue :type Boolean) (ElapsedSeconds :type Float%20%28double-precision%29) (TriggeredSeconds :type Float%20%28double-precision%29) (InputAction :type Input%20Action%20Object%20Reference :default "/Game/Blueprints/Controls/IA_Jump.IA_Jump"))
  ;[0.4385 0.5366 1] Activating the Character jump action with an input
  (:Started
    (Character|Jump))
  (:Completed
    (Character|StopJumping)))

(event Input|EnhancedActionEvents|EnhancedInputActionIA_Crouch
  (params (ActionValue :type Boolean) (ElapsedSeconds :type Float%20%28double-precision%29) (TriggeredSeconds :type Float%20%28double-precision%29) (InputAction :type Input%20Action%20Object%20Reference :default "/Game/Blueprints/Controls/IA_Crouch.IA_Crouch"))
  ;[1 0 0] Pressing Crouch to Toggle Crouch
  (:Triggered
    (CallFunction|ToggleCrouch true))
  (:Completed
    (CallFunction|ToggleCrouch false)))

(event Input|EnhancedActionEvents|EnhancedInputActionIA_Run
  (params (ActionValue :type Float%20%28double-precision%29) (ElapsedSeconds :type Float%20%28double-precision%29) (TriggeredSeconds :type Float%20%28double-precision%29) (InputAction :type Input%20Action%20Object%20Reference :default "/Game/Blueprints/Controls/IA_Run.IA_Run"))
  ;[0.4948 0.4948 0.4948] Moving BP_PlayerSprite on input
  (Pawn|Input|AddMovementInput "1.000000,0.000000,0.000000" ActionValue false))

(event Input|EnhancedActionEvents|EnhancedInputActionIA_Pause
  (params (ActionValue :type Boolean) (ElapsedSeconds :type Float%20%28double-precision%29) (TriggeredSeconds :type Float%20%28double-precision%29) (InputAction :type Input%20Action%20Object%20Reference :default "/Game/Blueprints/Controls/IA_Pause.IA_Pause"))
  (bind _returnvalue (Game|GetPlayerController 0))
  ;[0 0.2604 0.2258] Toggling the Pause Menu
  (:Started
    (if (Variables|Default|GetcanPause)
      (bind _returnvalue_2 (UserInterface|CreateWidget "/Game/Blueprints/PauseMenu.PauseMenu_C"))
      (bind _output_get (Variables|Default|SetPauseMenuReference _returnvalue_2))
      (Input|SetInputModeUIOnly _returnvalue _output_get "DoNotLock" false)
      (UserInterface|Viewport|AddtoViewport _output_get 0)
      (Variables|/Script/Engine.PlayerController|SetbShowMouseCursor _returnvalue true)
      (Game|SetGamePaused true))))

(event EventTick
  (params (DeltaSeconds :type Float%20%28single-precision%29))
  ;[0 0 0] Updating the anaimtion events on every tick
  (CallFunction|UpdateAnimation)
  (CallFunction|UpdateDirection))

(event EventBeginPlay
  ;[0 1 0.08472] Adding mapping context for Enhanced Input Actions
  (bind _asplayer_controller (Utilities|Casting|CastToPlayerController (Pawn|GetController)))
  (Utilities|IsValid (PlayerController|LocalPlayerSubsystems|GetEnhancedInputLocalPlayerSubsystem _asplayer_controller)
    (:Is%20Valid
      (Input|AddMappingContext (PlayerController|LocalPlayerSubsystems|GetEnhancedInputLocalPlayerSubsystem _asplayer_controller) "/Game/Blueprints/Controls/CustomEnhancedPlayerActionssss.CustomEnhancedPlayerActionssss" 0 "(bIgnoreAllPressedKeysUntilRelease=True,bForceImmediately=False,bNotifyUserSettings=False)")
      (Input|SetInputModeGameOnly (Game|GetPlayerController 0) false)
      (Variables|Default|SetcrouchSpeed (Variables|/Script/Engine.CharacterMovementComponent|GetMaxWalkSpeedCrouched (Variables|Character|GetCharacterMovement)))
      (Variables|Default|SetwalkSpeed (Variables|/Script/Engine.CharacterMovementComponent|GetMaxWalkSpeed (Variables|Character|GetCharacterMovement))))))

(fn ConstructionScript)